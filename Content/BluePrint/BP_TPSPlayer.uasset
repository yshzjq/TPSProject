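; Third-person shooter player Blueprint that handles the sniper UI overlay.
; BeginPlay creates and stores the WBP_SniperUI widget, which the IA_Sniper Enhanced Input action adds to the viewport when started and removes when completed.
; Bullet spawning at the FirePosition socket, controller-relative movement and disabling handgun collision remain only as disconnected nodes that never run.
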(event Input|EnhancedActionEvents|EnhancedInputActionIA_Sniper
  (params (ActionValue :type Boolean) (ElapsedSeconds :type Float%20%28double-precision%29) (TriggeredSeconds :type Float%20%28double-precision%29) (InputAction :type Input%20Action%20Object%20Reference :default "/Game/Input/IA_Sniper.IA_Sniper"))
  (bind _sniperui (Variables|Default|GetSniperUI))
  (:Started
    (UserInterface|Viewport|AddtoViewport _sniperui 0))
  (:Completed
    (Widget|RemovefromParent _sniperui)))

(event EventBeginPlay
  (bind _returnvalue (UserInterface|CreateWidget "/Game/BluePrint/WBP_SniperUI.WBP_SniperUI_C"))
  (Variables|Default|SetSniperUI _returnvalue))

(event Collision|EventActorBeginOverlap
  (params (OtherActor :type Actor%20Object%20Reference)))

(event EventTick
  (params (DeltaSeconds :type Float%20%28single-precision%29)))

(event Input|ActionEvents|InputActionFires
  (params (Key :type Key%20Structure :default "None")))

(fn ConstructionScript)